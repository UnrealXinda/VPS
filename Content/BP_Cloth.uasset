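; BP_Cloth is an actor that hosts a ProceduralCloth component and keeps its ground and sphere parameters current.
; Each Tick it sets GroundZ to the height of FloorActor relative to itself, and copies the Sphere component's scaled radius and relative location into the cloth.
; The construction script is empty, and its InitClothComponent call and sphere setup are left unconnected, so they never run.
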(event `self.ReceiveTick`
  (params (DeltaSeconds :type "Float (single-precision)"))
  (bind (_returnvalue_x _returnvalue_y _returnvalue_z) (`KismetMathLibrary.BreakVector` (`self.K2_GetActorLocation`)))
  (bind _proceduralcloth (`self.ProceduralCloth`))
  (bind _sphere (`self.Sphere`))
  (bind (_returnvalue_x_2 _returnvalue_y_2 _returnvalue_z_2) (`KismetMathLibrary.BreakVector` (`self.K2_GetActorLocation` (`self.FloorActor`))))
  (set `ProceduralClothComponent.GroundZ` (- _returnvalue_z_2 _returnvalue_z) _proceduralcloth)
  (set `ProceduralClothComponent.SphereRadius` (`SphereComponent.GetScaledSphereRadius` _sphere) _proceduralcloth)
  (set `ProceduralClothComponent.SphereLoc` (`SceneComponent.RelativeLocation` _sphere) _proceduralcloth))

(fn `UserConstructionScript`)